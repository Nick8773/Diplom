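; Side-scrolling 2D hero character that runs along world X with double jump, held dash, and light and heavy attacks.
; Jumps, landings and grounded attacks trigger animation-node jumps; landings and attacks also lock movement, with no unlock in this graph.
; Tick turns the controller to face the X velocity.
; Damage updates health, feeds the BeginPlay-created healthbar's change call, and knocks the hero away from EnemyPositionX or respawns it at its start.
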(event `InputAction|Jump`
  (params (Key :type "Key Structure"))
  (:`Pressed`
    (set `self.JumpMaxCount` 2)
    (set `self.JumpMaxHoldTime` 0.0)
    (`self.Jump`))
  (:`Released`
    (`self.StopJumping`)))

(event `InputAction|Dash`
  (params (Key :type "Key Structure"))
  (:`Pressed`
    (set `self.RunPlayRate` 1.5)
    (set `CharacterMovementComponent.MaxWalkSpeed` 1000.0 (`self.CharacterMovement`)))
  (:`Released`
    (set `self.RunPlayRate` 1.0)
    (set `CharacterMovementComponent.MaxWalkSpeed` 600.0 (`self.CharacterMovement`))))

(event `InputAxis|Forwford`
  (params (AxisValue :type "Float (single-precision)"))
  (if (not (`self.isMovmentLock`))
    (`self.AddMovementInput` (1.0 0.0 0.0) AxisValue)))

(event `self.OnJumped`
  (`PaperZDAnimInstance.JumpToNode` (`PaperZDAnimationComponent.AnimInstance` (`self.AnimationComponent`)) "Jump Action" "None" :!label _label))

(event `self.OnWalkingOffLedge`
  (params (PreviousFloorImpactNormal :type "Vector Structure (by ref)") (PreviousFloorContactNormal :type "Vector Structure (by ref)") (PreviousLocation :type "Vector Structure (by ref)") (TimeDelta :type "Float (single-precision)"))
  (goto _label))

(event `self.OnLanded`
  (params (Hit :type "HitResult Structure (by ref)"))
  (`PaperZDAnimInstance.JumpToNode` (`PaperZDAnimationComponent.AnimInstance` (`self.AnimationComponent`)) "Landed" "None")
  (`MovementComponent.StopMovementImmediately` (`self.CharacterMovement`))
  (set `self.isMovmentLock` true))

(event `self.ReceiveTick`
  (params (DeltaSeconds :type "Float (single-precision)"))
  (bind _returnvalue (`self.GetController`))
  (bind _returnvalue_2 (`self.GetController`))
  (bind _velocity_x (`KismetMathLibrary.BreakVector` (`MovementComponent.Velocity` (`self.CharacterMovement`))))
  (if (not (`self.isMovmentLock`))
    (`/Engine/EditorBlueprintResources/StandardMacros.CompareFloat` _velocity_x
      (:`>`
        (`/Engine/EditorBlueprintResources/StandardMacros.IsValid` _returnvalue
          (:`Is Valid`
            (`Controller.SetControlRotation` _returnvalue (`KismetMathLibrary.MakeRotator` 0.0)))))
      (:`<`
        (`/Engine/EditorBlueprintResources/StandardMacros.IsValid` _returnvalue_2
          (:`Is Valid`
            (`Controller.SetControlRotation` _returnvalue_2 (`KismetMathLibrary.MakeRotator` 0.0 0.0 180.0))))))))

(event `self.ReceiveBeginPlay`
  (set `self.Respawn Location` (`self.K2_GetActorLocation`))
  (bind _asplayer_controller (cast `PlayerController` (`self.GetController`)))
  (bind _returnvalue (`|CreateWidget` "/Game/blueprints/Hero/HUD/W_healthbar.W_healthbar_C" _asplayer_controller))
  (`UserWidget.AddToViewport` _returnvalue 0))

(event `self.ReceiveAnyDamage`
  (params (Damage :type "Float (single-precision)") (DamageType :type "DamageType Object Reference") (InstigatedBy :type "Controller Object Reference") (DamageCauser :type "Actor Object Reference"))
  (bind _returnvalue_x (`KismetMathLibrary.BreakVector` (`SceneComponent.K2_GetComponentLocation` (`self.Sprite`))))
  (if (not (`self.isDead`))
    (set `self.Health` (- (`self.Health`) Damage))
    (`KismetSystemLibrary.PrintString` (`KismetStringLibrary.Concat_StrStr` "Health: " (`KismetStringLibrary.Conv_DoubleToString` (`self.Health`))) true true (struct :`R` 1.0 :`G` 0.095909 :`A` 1.0))
    (`self.changinghealth` (/ (`self.Health`) (`self.Maxhealth`)))
    (if (> (`self.Health`) 0.0)
      (`/Engine/EditorBlueprintResources/StandardMacros.CompareFloat` _returnvalue_x (`self.EnemyPositionX`)
        (:`>`
          (`self.LaunchCharacter` (1000.0 0.0 50.0) true))
        (:`<`
          (`self.LaunchCharacter` (-1000.0 0.0 50.0) true)))
      (else
        (set `self.isDead` true)
        (`ActorComponent.SetActive` (`self.CharacterMovement`) false false)
        (`KismetSystemLibrary.Delay` 1.0)
        (`self.Respawn`)))))

(event `Respawn`
  (`self.K2_SetActorLocation` (`self.Respawn Location`))
  (set `self.isDead` false)
  (`ActorComponent.SetActive` (`self.CharacterMovement`) true false)
  (set `self.Health` 100.0))

(event `InputAction|LightAttack`
  (params (Key :type "Key Structure"))
  (:`Pressed`
    (if (and (not (`self.isAttacking`)) (`NavMovementInterface.IsMovingOnGround` (`self.CharacterMovement`)))
      (set `self.isAttacking` true)
      (`PaperZDAnimInstance.JumpToNode` (`PaperZDAnimationComponent.AnimInstance` (`self.AnimationComponent`)) "LightAttack" "None")
      (`MovementComponent.StopMovementImmediately` (`self.CharacterMovement`))
      (set `self.isMovmentLock` true)
      (`KismetSystemLibrary.Delay` 0.5)
      (set `self.isAttacking` false))))

(event `InputAction|HeavyAttack`
  (params (Key :type "Key Structure"))
  (:`Pressed`
    (if (and (not (`self.isAttacking`)) (`NavMovementInterface.IsMovingOnGround` (`self.CharacterMovement`)))
      (set `self.isAttacking` true)
      (`PaperZDAnimInstance.JumpToNode` (`PaperZDAnimationComponent.AnimInstance` (`self.AnimationComponent`)) "HeavyAttack" "None")
      (`MovementComponent.StopMovementImmediately` (`self.CharacterMovement`))
      (set `self.isMovmentLock` true)
      (`KismetSystemLibrary.Delay` 0.5)
      (set `self.isAttacking` false))))

(fn `UserConstructionScript`)